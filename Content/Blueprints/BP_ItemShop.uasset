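; BP_ItemShop is a purchasable item actor that the player buys with collected coins by walking into it.
; On BeginPlay it writes its ItemCost into the Cost text display.
; When BP_ThirdPersonCharacterCustom overlaps the Box with enough CoinsCollected, it subtracts the cost from that character and destroys itself, without granting anything else.
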(event `self.ReceiveBeginPlay`
  (`TextRenderComponent.K2_SetText` (`self.Cost`) (`KismetTextLibrary.Conv_StringToText` (`KismetStringLibrary.BuildString_Int` "" "Costs " (`self.ItemCost`) " Coins!"))))

(event `self.Box.OnComponentBeginOverlap`
  (params (OverlappedComponent :type "PrimitiveComponent Object Reference") (OtherActor :type "Actor Object Reference") (OtherComp :type "PrimitiveComponent Object Reference") (OtherBodyIndex :type Integer) (bFromSweep :type Boolean) (SweepResult :type "HitResult Structure (by ref)"))
  (bind _itemcost (`self.ItemCost`))
  (bind _asbp_third_person_character_custom (cast `/Game/Blueprints/BP_ThirdPersonCharacterCustom` OtherActor))
  (bind _coinscollected (`/Game/Blueprints/BP_ThirdPersonCharacterCustom.CoinsCollected` _asbp_third_person_character_custom))
  (if (>= _coinscollected _itemcost)
    (set `/Game/Blueprints/BP_ThirdPersonCharacterCustom.CoinsCollected` (- _coinscollected _itemcost) _asbp_third_person_character_custom)
    (`self.K2_DestroyActor`)))

(fn `UserConstructionScript`)