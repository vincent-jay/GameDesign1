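; BP_FinishTime is a finish-line trigger that times the player's laps.
; BeginPlay creates the W_FinishLineTimer widget and starts a self-recalling Delay loop, used instead of Tick, that shows current lap time on the widget and as a debug print.
; When BP_ThirdPersonCharacterCustom enters the Box, it prints the lap time and resets the real-time timestamp that the loop measures from.
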(event `self.ReceiveBeginPlay`
  (bind _returnvalue (`|CreateWidget` "/Game/Widgets/W_FinishLineTimer.W_FinishLineTimer_C"))
  (bind _output_get (set `self.W_TimerWidget` _returnvalue))
  (`UserWidget.AddToViewport` _output_get 0)
  (`self.On Screen Timer`))

(event `On Screen Timer`
  (bind _returnvalue (`KismetStringLibrary.Concat_StrStr` "Current lap: " (`KismetTextLibrary.Conv_TextToString` (`KismetTextLibrary.Conv_DoubleToText` (- (`GameplayStatics.GetRealTimeSeconds`) (`self.LastTimestamp`)) "HalfToEven" false true 1 324 2 2)) " seconds!"))
  (`KismetSystemLibrary.PrintString` _returnvalue true true (struct :`G` 0.66 :`B` 1.0 :`A` 1.0) 0.01)
  (`TextBlock.SetText` (`/Game/Widgets/W_FinishLineTimer.CurrentTimeText` (`self.W_TimerWidget`)) (`KismetTextLibrary.Conv_StringToText` _returnvalue))
  (`KismetSystemLibrary.Delay` 0.01)
  (`self.On Screen Timer`))

(event `self.Box.OnComponentBeginOverlap`
  (params (OverlappedComponent :type "PrimitiveComponent Object Reference") (OtherActor :type "Actor Object Reference") (OtherComp :type "PrimitiveComponent Object Reference") (OtherBodyIndex :type Integer) (bFromSweep :type Boolean) (SweepResult :type "HitResult Structure (by ref)"))
  (cast `/Game/Blueprints/BP_ThirdPersonCharacterCustom` OtherActor)
  (`KismetSystemLibrary.PrintString` (`KismetStringLibrary.Concat_StrStr` "That lap took " (`KismetTextLibrary.Conv_TextToString` (`KismetTextLibrary.Conv_DoubleToText` (- (`GameplayStatics.GetRealTimeSeconds`) (`self.LastTimestamp`)) "HalfToEven" false true 1 324 0 2)) " seconds!"))
  (set `self.LastTimestamp` (`GameplayStatics.GetRealTimeSeconds`)))

(fn `UserConstructionScript`)